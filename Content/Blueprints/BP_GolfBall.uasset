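; BP_GolfBall is a player-controllable golf ball that launches itself when a shot is taken.
; The DoShot event ignores power at or below a minimum, caps it at a maximum, and applies it as a physics impulse to the static mesh.
; The shot direction is the forward vector of the controller's control rotation.
; BeginPlay, Tick and the construction script are empty.
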(event `self.ReceiveBeginPlay`)

(event `self.ReceiveTick`
  (params (DeltaSeconds :type "Float (single-precision)")))

(event `self.DoShot`
  (params (ShotPower :type "Float (single-precision)"))
  (if (> ShotPower (`self.MinShotPower`))
    (`PrimitiveComponent.AddImpulse` (`self.StaticMesh`) (* (`KismetMathLibrary.GetForwardVector` (`Controller.GetControlRotation` (`self.GetController`))) (`KismetMathLibrary.FClamp` ShotPower 0.0 (`self.MaxShotPower`))) "None" false)))

(fn `UserConstructionScript`)