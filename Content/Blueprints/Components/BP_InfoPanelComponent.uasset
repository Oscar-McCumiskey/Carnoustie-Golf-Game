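; BP_InfoPanelComponent is an actor component that shows an informational title and body panel to the player in the golf game.
; Its DisplayInfoPanel event looks up the component on the passed actor and reads its InfoPanelData asset.
; It sends that text to the BP_GolfGamePlayerController for display and plays a bell sound.
; A missing component or data asset prints a debug message naming the actor.
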(event `DisplayInfoPanel`
  (params (InfoPanelActor :type "Actor Object Reference") (Controller :type "Controller Object Reference"))
  (bind _returnvalue (`KismetSystemLibrary.GetDisplayName` InfoPanelActor))
  (bind _returnvalue_2 (`Actor.GetComponentByClass` InfoPanelActor "BP_InfoPanelComponent_C"))
  (`/Engine/EditorBlueprintResources/StandardMacros.IsValid` _returnvalue_2
    (:`Is Valid`
      (bind _infopaneldata (`/Game/Blueprints/Components/BP_InfoPanelComponent.InfoPanelData` _returnvalue_2)
        (:`then`
          (bind _asbp_golf_game_player_controller (cast `/Game/Blueprints/Player/BP_GolfGamePlayerController` Controller))
          (`/Game/Blueprints/Player/BP_GolfGamePlayerController.DisplayInfoPanel` _asbp_golf_game_player_controller (`/Game/Blueprints/UI/InformationPanels/TextData/DA_InfoPanelData.InfoPanelTitle` _infopaneldata) (`/Game/Blueprints/UI/InformationPanels/TextData/DA_InfoPanelData.InfoPanelBody` _infopaneldata))
          (`GameplayStatics.PlaySound2D` "/Game/Assets/Sounds/MS_BellDing.MS_BellDing" 1.0 1.0 0.0 null null))
        (:`else`
          (`KismetSystemLibrary.PrintString` (`KismetStringLibrary.Concat_StrStr` _returnvalue ": No Data Asset") true true (struct :`R` 1.0 :`A` 1.0) 10.0))))
    (:`Is Not Valid`
      (`KismetSystemLibrary.PrintString` (`KismetStringLibrary.Concat_StrStr` _returnvalue ": Info Panel Missing Component") true true (struct :`R` 1.0 :`A` 1.0) 10.0))))