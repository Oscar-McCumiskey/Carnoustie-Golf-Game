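; BP_InfoPanelRing is a ring actor that marks itself as triggered when the player overlaps it.
; BeginPlay creates a dynamic material on the Visual component and rotates the minimap icon to a fixed orientation.
; An overlap from a Player-tagged actor, gated by HasTriggered, turns the material and minimap sprite green, plays the InfoPanelAppear sound and sets that flag.
; The file itself contains no logic for displaying an info panel.
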(event `self.ReceiveBeginPlay`
  (bind _visual (`self.Visual`))
  (bind _returnvalue (`PrimitiveComponent.CreateDynamicMaterialInstance` _visual 0 (`PrimitiveComponent.GetMaterial` _visual 0) "None"))
  (set `self.DynamicMaterial` _returnvalue)
  (`SceneComponent.K2_SetWorldRotation` (`self.MinimapIcon`) (struct :`Roll` 90.0) false false))

(event `self.ReceiveActorBeginOverlap`
  (params (OtherActor :type "Actor Object Reference"))
  (`self.HasTriggered`
    (:`then`)
    (:`else`
      (if (`self.ActorHasTag` OtherActor "Player")
        (`self.PlayerTriggered`)))))

(event `PlayerTriggered`
  (`MaterialInstanceDynamic.SetVectorParameterValue` (`self.DynamicMaterial`) "Colour" (struct :`G` 1.0 :`A` 1.0))
  (`GameplayStatics.PlaySound2D` "/Game/Assets/Sounds/Ques/InfoPanelAppear.InfoPanelAppear" 1.0 1.0 0.0 null null)
  (`PaperSpriteComponent.SetSpriteColor` (`self.MinimapIcon`) (struct :`G` 1.0 :`A` 1.0))
  (set `self.HasTriggered` true))

(fn `UserConstructionScript`)