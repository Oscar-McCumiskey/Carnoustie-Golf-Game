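; Cinematic camera actor that starts on BeginPlay, takes camera control from the golf pawn and flies through placed target nodes.
; Node locations become InterpToMovement control points for the path.
; NextNode advances the index and runs a Rotate timeline that lerps from the camera's current rotation toward that node's rotation.
; Near the list's end, it waits briefly, then stops the cinematic, restoring the pawn's camera.
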(event `self.ReceiveBeginPlay`
  (`self.StartCinematic`))

(event `self.OnStartCinematic`
  (bind _asbp_golf_pawn_legacy (cast `/Game/Blueprints/Player/Deprecated/BP_GolfPawnLegacy` (`GameplayStatics.GetPlayerPawn` 0)))
  (`/Game/Blueprints/Player/Deprecated/BP_GolfPawnLegacy.TakeCameraControl` _asbp_golf_pawn_legacy self)
  (set `self.CurNodeIndex` 0)
  (for _array_element (`self.TargetNodes`)
    (`InterpToMovementComponent.AddControlPointPosition` (`self.InterpToMovement`) (`self.K2_GetActorLocation` _array_element) false))
  (`InterpToMovementComponent.FinaliseControlPoints` (`self.InterpToMovement`))
  (`self.NextNode`))

(event `NextNode`
  (bind _targetnodes (`self.TargetNodes`))
  (bind _result (`/Engine/EditorBlueprintResources/StandardMacros.IncrementInt` (`self.CurNodeIndex`))
    (:`  `
      (bind _output_get (set `self.CurNode` (`|GetArrayItem` _targetnodes _result)))
      (if (>= (`self.CurNodeIndex`) (- (`KismetArrayLibrary.Array_Length` _targetnodes) 1))
        (`KismetSystemLibrary.Delay` 3.0)
        (`self.StopCinematic`)
        (else
          (set `self.TargetRotation` (`self.K2_GetActorRotation` _output_get))
          (`|ExecutionSequence`
            (:`then_0`
              (bind (_direction _time) (`Timeline|Rotate` :!via `SetNewTime` :!label _label)
                (:`Update`
                  (`SceneComponent.K2_SetRelativeRotation` (`self.Camera`) (`KismetMathLibrary.RLerp` (`SceneComponent.RelativeRotation` (`self.Camera`)) (`self.TargetRotation`) _time) false false))))
            (:`then_1`
              (goto _label :!via `PlayFromStart`))))))))

(event `self.OnStopCinematic`
  (bind _asbp_golf_pawn_legacy (cast `/Game/Blueprints/Player/Deprecated/BP_GolfPawnLegacy` (`GameplayStatics.GetPlayerPawn` 0)))
  (`/Game/Blueprints/Player/Deprecated/BP_GolfPawnLegacy.RestoreCamera` _asbp_golf_pawn_legacy true))

(fn `UserConstructionScript`)