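; Water body actor that plays a hit effect on contact and tracks whether the player's golf ball is in the water.
; BeginPlay caches the player pawn as a BP_GolfBall.
; Any overlapping actor spawns a water-hit effect at its location with a fixed maximum velocity.
; Only the cached ball has its IsInWater flag set on begin overlap and cleared on end overlap.
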(event `self.ReceiveBeginPlay`
  (bind _asbp_golf_ball (cast `/Game/Blueprints/Player/BP_GolfBall` (`GameplayStatics.GetPlayerPawn` 0)))
  (set `self.GolfBall` _asbp_golf_ball))

(event `self.ReceiveActorBeginOverlap`
  (params (OtherActor :type "Actor Object Reference"))
  (bind _returnvalue (`NiagaraFunctionLibrary.SpawnSystemAtLocation` "/Game/Blueprints/Particles/FXS_WaterHit.FXS_WaterHit" (`self.K2_GetActorLocation` OtherActor)))
  (`NiagaraComponent.SetVariableFloat` _returnvalue "MaximumVelocity" 1000.0)
  (if (== OtherActor (`self.GolfBall`))
    (set `/Game/Blueprints/Player/BP_GolfBall.IsInWater` true (`self.GolfBall`))))

(event `self.ReceiveActorEndOverlap`
  (params (OtherActor :type "Actor Object Reference"))
  (if (== OtherActor (`self.GolfBall`))
    (set `/Game/Blueprints/Player/BP_GolfBall.IsInWater` false (`self.GolfBall`))))

(fn `UserConstructionScript`)