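; BP_OutOfBound is an overlap-triggered actor that sends a BP_GolfBall out of bounds.
; On overlap by the ball, it plays a trigger sound at the ball's location and waits briefly so the sound can play.
; It then calls the ball's OutOfBounds with its OOB type and custom text.
; A CanTrigger flag is cleared during the delay and restored afterwards to guard against repeat triggers.
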(event `self.ReceiveBeginPlay`
  (set `self.CanTrigger` true))

(event `self.ReceiveActorBeginOverlap`
  (params (OtherActor :type "Actor Object Reference"))
  (`self.CanTrigger`
    (:`then`
      (bind _asbp_golf_ball (cast `/Game/Blueprints/Player/BP_GolfBall` OtherActor))
      (set `self.CanTrigger` false)
      (`GameplayStatics.PlaySoundAtLocation` (`self.SoundOnTrigger`) (`self.K2_GetActorLocation` _asbp_golf_ball) (struct) 1.0 1.0 0.0 null null null null)
      (`KismetSystemLibrary.Delay` 1.25) ; Delay to make way for any sounds
      (`/Game/Blueprints/Player/BP_GolfBall.OutOfBounds` _asbp_golf_ball (`self.OOBType`) (`self.CustomText`))
      (set `self.CanTrigger` true))
    (:`else`)))

(fn `UserConstructionScript`)