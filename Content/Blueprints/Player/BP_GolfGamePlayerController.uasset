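; Player controller for a golf game that handles club selection, shot charging and hitting the controlled golf ball.
; Club cycling pulls power, angle, charge curve and swing sounds from club data and updates the HUD.
; A looping timer started on possess previews the trajectory with debug-drawn projectile prediction until the shot.
; Shots launch along control yaw at the club's angle, with light or heavy sounds chosen by charged power.
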(event `self.ReceiveBeginPlay`
  (set `self.bShowMouseCursor` true)
  (`WidgetBlueprintLibrary.SetInputMode_GameAndUIEx` self null "DoNotLock" false)
  (bind _asbp_golf_ball (cast `/Game/Blueprints/Player/BP_GolfBall` (`self.K2_GetPawn`)))
  (set `self.GolfBall` _asbp_golf_ball)
  ;[0 0.02279 0.15 0.5] Delayed Initialise
  (`KismetSystemLibrary.DelayUntilNextTick`)
  (`self.CycleGolfClub` 0)
  (set `self.CurrentShotPower` (`CurveFloat.GetFloatValue` (`self.CurrentShotPowerCurve`) (`self.MinimumShotChargeTime`))))

(event `BeginGolfShot`
  (bind _minimumshotchargetime (`self.MinimumShotChargeTime`))
  (set `self.CurrentShotPower` (`CurveFloat.GetFloatValue` (`self.CurrentShotPowerCurve`) _minimumshotchargetime))
  (set `self.CurrentShotTime` _minimumshotchargetime)
  (`KismetSystemLibrary.PrintString` "Hello"))

(event `ChargeGolfShot`
  (params (DeltaTime :type "Float (double-precision)"))
  (`self.UpdateShotPower` DeltaTime (`self.CurrentShotPowerCurve`)))

(event `self.ReceivePossess`
  (params (PossessedPawn :type "Pawn Object Reference"))
  (`self.StartDrawingTrajectory`))

(event `ExecuteGolfShotShot`
  (bind _golfball (`self.GolfBall`))
  (if (>= (`self.CurrentShotPower`) (/ (`CurveFloat.GetFloatValue` (`self.CurrentShotPowerCurve`) (`self.MaximumShotChargeTime`)) 1.5))
    (`/Game/Blueprints/Player/BP_GolfBall.BallSwung` _golfball (`self.HeavySwingSnds`)) ; High power shot
    (else
      (`/Game/Blueprints/Player/BP_GolfBall.BallSwung` _golfball (`self.LightSwingSnds`)) ; Low power shot
    ))
  (`self.Shoot` (* (`self.CurrentShotPower`) (`self.ShotMultiplier`) (`self.GolfClubShotPower`)) (`self.CurrentShotAngle`))
  (set `self.CurrentShotPower` (`CurveFloat.GetFloatValue` (`self.CurrentShotPowerCurve`) (`self.MinimumShotChargeTime`))))

(event `StartDrawingTrajectory`
  (bind _returnvalue (`KismetSystemLibrary.K2_SetTimerDelegate` (delegate `Trajectory`) 0.01 true true))
  (set `self.TrajectoryHandle` _returnvalue))

(event `Trajectory`
  (`self.DrawProjectilePath` true (* (`self.CurrentShotPower`) (`self.ShotMultiplier`) (`self.GolfClubShotPower`)) (`self.CurrentShotAngle`) 5.0 "ForOneFrame"))

(event `Shoot`
  (params (ShotPower :type "Float (double-precision)") (ShotAngle :type "Float (double-precision)"))
  (bind (_returnvalue_roll _returnvalue_pitch _returnvalue_yaw) (`KismetMathLibrary.BreakRotator` (`self.GetControlRotation`)))
  (bind _golfball (`self.GolfBall`))
  (`PrimitiveComponent.SetSimulatePhysics` (`GolfBallPawn.StaticMesh` _golfball) true)
  (`GolfBallPawn.DoShot` _golfball (`KismetMathLibrary.GetForwardVector` (`KismetMathLibrary.MakeRotator` _returnvalue_roll ShotAngle _returnvalue_yaw)) ShotPower (- (`self.K2_GetActorLocation` (`self.GolfBall`)) (0.0 0.0 10.0)))
  (`KismetSystemLibrary.K2_ClearAndInvalidateTimerHandle` (`self.TrajectoryHandle`))
  (`self.DrawProjectilePath` true ShotPower ShotAngle 10.0 "ForDuration" 10.0))

(fn `CycleGolfClub`
  (params (Increment :type Integer))
  (bind (_output_displayname _output_staticmesh _output_imagetexture2d _output_swingpower _output_hitangle _output_shotpowercurve _output_lightswingsounds _output_heavyswingsounds) (break `/Game/Blueprints/Structures/S_GolfClubs` (`|GetArrayItem` (`/Game/Blueprints/UI/GolfClubSelection/GolfClubData/DA_GolfClubs.GolfClubs` (`self.GolfClubData`)) (`self.GolfClubIndex`))))
  (bind _output_get (set `self.GolfClubIndex` (+ Increment (`self.GolfClubIndex`))))
  (`self.RealWrapIntegerInclusive` _output_get 0 (- (`KismetArrayLibrary.Array_Length` (`/Game/Blueprints/UI/GolfClubSelection/GolfClubData/DA_GolfClubs.GolfClubs` (`self.GolfClubData`))) 1))
  (bind _asplayer_hud (cast `/Game/Blueprints/UI/PlayerHUD` (`self.GetHUD`)))
  (`/Game/Blueprints/UI/GolfClubSelection/W_ClubSelector.SetClubDetails` (`/Game/Blueprints/UI/PlayerHUD.ClubSelectorHUD` _asplayer_hud) _output_imagetexture2d (`KismetTextLibrary.Conv_NameToText` _output_displayname))
  (set `self.GolfClubShotPower` _output_swingpower)
  (set `self.CurrentShotAngle` _output_hitangle)
  (bind _output_get_2 (set `self.CurrentShotPowerCurve` _output_shotpowercurve))
  (set `self.CurrentShotPower` (`CurveFloat.GetFloatValue` _output_get_2 (`self.MinimumShotChargeTime`)))
  (set `self.LightSwingSnds` _output_lightswingsounds)
  (set `self.HeavySwingSnds` _output_heavyswingsounds))

(fn `DisplayInfoPanel`
  (params (Title :type Text) (Body :type Text))
  (bind _asplayer_hud (cast `/Game/Blueprints/UI/PlayerHUD` (`self.GetHUD`)))
  (`/Game/Blueprints/UI/InformationPanels/W_InfoPanelWidget.DisplayInfoPanel` (`/Game/Blueprints/UI/PlayerHUD.InfoPanelHUD` _asplayer_hud) Title Body))

(fn `DrawProjectilePath`
  (params (DrawPath :type Boolean) (ShotPower :type "Float (double-precision)") (ShotAngle :type "Float (double-precision)") (SimTime :type "Float (double-precision)") (DebugType :type "EDrawDebugTrace Enum" :default "None") (DrawDuration :type "Float (double-precision)"))
  (bind (_returnvalue_roll _returnvalue_pitch _returnvalue_yaw) (`KismetMathLibrary.BreakRotator` (`self.GetControlRotation`)))
  (if DrawPath
    (`GameplayStatics.Blueprint_PredictProjectilePath_Advanced` (make `PredictProjectilePathParams` (`SceneComponent.K2_GetComponentLocation` (`GolfBallPawn.StaticMesh` (`self.GolfBall`))) (* (`KismetMathLibrary.GetForwardVector` (`KismetMathLibrary.MakeRotator` _returnvalue_roll ShotAngle _returnvalue_yaw)) 20 ShotPower) false 0.0 SimTime true "ECC_PhysicsBody" _ (`|MakeArray` self :!type "Actor Object Reference") 20.0 0.0 DebugType DrawDuration))))

(fn `RealWrapIntegerInclusive`
  (params (Value :type "Integer (by ref)") (Min :type Integer) (Max :type Integer))
  (`|ExecutionSequence`
    (:`then_0`
      (if (< Value Min)
        (`|VariableSetRef` Value Max)))
    (:`then_1`
      (if (> Value Max)
        (`|VariableSetRef` Value Min)))))

(fn `UserConstructionScript`)