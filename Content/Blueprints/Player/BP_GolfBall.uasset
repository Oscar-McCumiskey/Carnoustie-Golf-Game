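; BP_GolfBall is the player's physics-driven golf ball, handling each shot from aim preview and club spawning to stop or out-of-bounds reset.
; A looping timer applies wind, accuracy force and a speed cap, completing the shot once the grounded ball stays slow.
; Hit events drive surface-based sounds and progressive damping via physical materials and a velocity curve.
; Spline meshes draw trajectory and minimap prediction; collected info panels display after shots.
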(event `DoTrajectorySpline`
  (params (Points :type "Array of Vector Structure"))
  ;[0.7969 0.7969 0.7969 0.5] Trajectory Spline
  (set `self.TrajectoryPoints` Points)
  (`self.ClearSpline`)
  (for _array_element (`self.TrajectoryPoints`)
    (`SplineComponent.AddSplinePoint` (`self.TrajectorySpline`) _array_element "Local" true))
  (`SplineComponent.SetSplinePointType` (`self.TrajectorySpline`) 0 "CurveClamped" true)
  (for _index (range (`SplineComponent.GetNumberOfSplinePoints` (`self.TrajectorySpline`)))
    (bind _returnvalue (`AddComponent|NODE_AddSplineMeshComponent-5` :`bManualAttachment` true))
    (`PrimitiveComponent.SetHiddenInSceneCapture` _returnvalue true)
    (`PrimitiveComponent.SetCastShadow` _returnvalue false)
    (`KismetArrayLibrary.Array_Add` (`self.SplineMeshes`) _returnvalue)
    (bind (_location _tangent) (`SplineComponent.GetLocationAndTangentAtSplinePoint` (`self.TrajectorySpline`) _index "Local"))
    (bind (_location_2 _tangent_2) (`SplineComponent.GetLocationAndTangentAtSplinePoint` (`self.TrajectorySpline`) (+ _index 1) "Local"))
    (`SplineMeshComponent.SetStartAndEnd` _returnvalue _location _tangent _location_2 _tangent_2 true)))

(event `ClearSpline`
  (bind _splinemeshes (`self.SplineMeshes`))
  ;[0.7969 0.7969 0.7969 0.5] Trajectory Spline
  (`ActorComponent.K2_DestroyComponent` _splinemeshes)
  (`KismetArrayLibrary.Array_Clear` _splinemeshes)
  (`SplineComponent.ClearSplinePoints` (`self.TrajectorySpline`) true))

(event `OutOfBounds`
  ;[1 0 0 0.5] Out of Bounds
  (`self.K2_SetActorTransform` (`self.LastTransform`) false true)
  (`PrimitiveComponent.SetSimulatePhysics` (`self.StaticMesh`) false)
  (`self.GolfComplete`))

(event `self.ReceiveBeginPlay`
  ;[0.3218 0.7865 0.000267 0.5] Begin Setup
  (set `self.LastTransform` (`self.GetTransform`))
  (bind _asbp_golf_game_player_controller (cast `/Game/Blueprints/Player/BP_GolfGamePlayerController` (`self.GetController`)))
  (set `self.GolfController` _asbp_golf_game_player_controller)
  (bind _asbp_golf_game_mode (cast `/Game/Blueprints/BP_GolfGameMode` (`GameplayStatics.GetGameMode`)))
  (set `self.GolfGame` _asbp_golf_game_mode)
  (bind _returnvalue (`|CreateWidget` "/Game/Blueprints/UI/Trivia/W_Trivia.W_Trivia_C" (`GameplayStatics.GetPlayerController` 0)))
  (bind _output_get (set `self.TriviaWidget` _returnvalue))
  (`UserWidget.AddToViewport` _output_get 0)
  (`Widget.SetVisibility` _output_get "Hidden")
  (`self.SpawnGolfClub`))

(event `PlayImpactSound`
  (params (VolumeMulti :type "Float (double-precision)") (PhysMat :type "PhysicalMaterial Object Reference"))
  ;[1 0.9734 0 0.8] Play impact sound
  (bind _sound (`self.GetSoundFromPhysMat` PhysMat))
  (`GameplayStatics.PlaySoundAtLocation` _sound (`SceneComponent.K2_GetComponentLocation` (`self.StaticMesh`)) (struct) VolumeMulti 1.0 0.0 null null null null))

(event `TryImpact`
  (params (Impact :type "Vector Structure") (PhysMat :type "PhysicalMaterial Object Reference"))
  (bind _returnvalue (`KismetMathLibrary.VSize` Impact))
  ;[1 0.9734 0 0.8] Try to do impact sound
  (if (> _returnvalue 25.0)
    (`self.PlayImpactSound` (`KismetMathLibrary.FClamp` (/ _returnvalue 100.0) 0.0 1.5) PhysMat)))

(event `BallSwung`
  (params (Sound :type "SoundWave Object Reference"))
  ;[0 0.75 0.6965 0.5] Ball Swung
  (`GameplayStatics.PlaySoundAtLocation` Sound (`SceneComponent.K2_GetComponentLocation` (`self.StaticMesh`)) (struct) 1.0 1.0 0.0 null null null null)
  (set `self.BallFloored` false)
  (bind _output_get (set `self.BallStoppingForce` (`self.BallBaseStoppingForce`)))
  (`PrimitiveComponent.SetLinearDamping` (`self.StaticMesh`) _output_get)
  (`PrimitiveComponent.SetAngularDamping` (`self.StaticMesh`) 1.0)
  (set `self.GroundFrictionTimer` 0.0)
  (`self.ClearSpline`)
  (bind _returnvalue (`KismetSystemLibrary.K2_SetTimerDelegate` (delegate `GolfActive`) 0.001 true true))
  (set `self.GolfActiveHandle` _returnvalue))

(event `CreatePredictSpline`
  (params (GolfClub :type "/Game/Blueprints/Structures/S_GolfClubs Structure"))
  ;[0.849 0.849 0.849 0.5] Predict Spline
  (set `self.GolfClubData` GolfClub))

(event `GolfActive`
  (bind _staticmesh (`self.StaticMesh`))
  (bind _returnvalue (`SceneComponent.GetComponentVelocity` _staticmesh))
  ; Golf ball active
  (`self.IsInWorld`
    (:`Inside`
      (if (>= (`KismetMathLibrary.VSize` _returnvalue) 6000.0)
        (`PrimitiveComponent.SetPhysicsLinearVelocity` _staticmesh (* (`KismetMathLibrary.Normal` _returnvalue) 6000.0) false "None"))
      (`self.IsGrounded`
        (:`True`
          (set `self.BallFloored` true)
          (if (< (`KismetMathLibrary.VSize` (`SceneComponent.GetComponentVelocity` (`self.StaticMesh`))) 10.0)
            (if (not (`KismetSystemLibrary.K2_IsTimerActiveHandle` (`self.GolfStopHandle`)))
              (bind _returnvalue_2 (`KismetSystemLibrary.K2_SetTimerDelegate` (delegate `GolfComplete`) 1.0))
              (set `self.GolfStopHandle` _returnvalue_2))
            (else
              (`KismetSystemLibrary.K2_ClearAndInvalidateTimerHandle` (`self.GolfStopHandle`)))))
        (:`False`
          (set `self.BallFloored` false)
          (`/Game/Blueprints/BP_GolfGameMode.IsWindEnabled` (`self.GolfGame`)
            (:`then`
              (`PrimitiveComponent.AddForce` (`self.StaticMesh`) (* (`self.WindDirection`) (`self.WindPower`)) "None" false))
            (:`else`
              _))
          (`PrimitiveComponent.AddForce` (`self.StaticMesh`) (`/Game/Blueprints/Player/BP_GolfGamePlayerController.AccuracyVector` (`self.GolfController`)) "None" false))))
    (:`Outside`
      (`self.OutOfBounds`))))

(event `UpdatePredictSpline`
  (bind _minimappredictspline (`self.MinimapPredictSpline`))
  (bind _minimappredictspline_2 (`self.MinimapPredictSpline`))
  (bind (_golfclubdata_displayname _golfclubdata_mesh _golfclubdata_imagetexture2d _golfclubdata_swingpower) (break `/Game/Blueprints/Structures/S_GolfClubs` (`self.GolfClubData`)))
  (bind (_returnvalue_x _returnvalue_y) (`KismetMathLibrary.BreakVector` (`SceneComponent.GetForwardVector` (`self.Camera`))))
  (bind (_location _tangent) (`SplineComponent.GetLocationAndTangentAtSplinePoint` _minimappredictspline_2 0 "Local"))
  (bind (_location_2 _tangent_2) (`SplineComponent.GetLocationAndTangentAtSplinePoint` _minimappredictspline_2 1 "Local"))
  (bind _returnvalue (+ (`SceneComponent.K2_GetComponentLocation` (`self.StaticMesh`)) (* (`KismetMathLibrary.Vector_Up`) 1024)))
  ;[0.849 0.849 0.849 0.5] Predict Spline
  (`/Game/Blueprints/Player/BP_GolfGamePlayerController.CanShoot` (`self.GolfController`)
    (:`then`
      (bind _predictsplinemesh (`self.PredictSplineMesh`)
        (:`then`
          (`ActorComponent.K2_DestroyComponent` _predictsplinemesh))
        (:`else`
          _))
      (`SplineComponent.ClearSplinePoints` _minimappredictspline true)
      (`SplineComponent.AddSplinePoint` _minimappredictspline _returnvalue "Local" true)
      (`SplineComponent.AddSplinePoint` (`self.MinimapPredictSpline`) (+ _returnvalue (* (`KismetMathLibrary.MakeVector` _returnvalue_x _returnvalue_y) (* _golfclubdata_swingpower 2048.0))) "Local" true)
      (bind _returnvalue_2 (`AddComponent|NODE_AddSplineMeshComponent-4` :`bManualAttachment` true))
      (bind _output_get (set `self.PredictSplineMesh` _returnvalue_2))
      (`PrimitiveComponent.SetOwnerNoSee` _output_get true)
      (`PrimitiveComponent.SetCastShadow` _output_get false)
      (`SplineMeshComponent.SetStartAndEnd` _output_get _location _tangent _location_2 _tangent_2 true))
    (:`else`
      (bind _predictsplinemesh_2 (`self.PredictSplineMesh`)
        (:`then`
          (`ActorComponent.K2_DestroyComponent` _predictsplinemesh_2))
        (:`else`)))))

(event `self.StaticMesh.OnComponentHit`
  (params (HitComponent :type "PrimitiveComponent Object Reference") (OtherActor :type "Actor Object Reference") (OtherComp :type "PrimitiveComponent Object Reference") (NormalImpulse :type "Vector Structure") (Hit :type "HitResult Structure (by ref)"))
  (`self.TryImpact` NormalImpulse Hit_PhysMat)
  (`PrimitiveComponent.SetLinearDamping` (`self.StaticMesh`) (`self.BallStoppingForce`))
  (`PrimitiveComponent.SetAngularDamping` (`self.StaticMesh`) (`KismetMathLibrary.FMax` (`self.BallStoppingForce`) 1.0))
  (`|ExecutionSequence`
    (:`then_0`
      (`self.UpdateGolfBallDamping` Hit_PhysMat))
    (:`then_1`
      (set `self.CurrentGolfBallSurface` (`BlueprintMapLibrary.Map_Find` (`self.PhysicsMaterialMap`) Hit_PhysMat)))))

(event `GolfComplete`
  ; Golf ball active
  (`self.ShotComplete`)
  (`self.IsInputsLocked`
    (:`Locked`
      (bind _golfclub (`self.GolfClub`)
        (:`then`
          (`self.K2_DestroyActor` _golfclub))
        (:`else`)))
    (:`Unlocked`
      (`self.SpawnGolfClub`)
      (`/Game/Blueprints/Player/BP_GolfGamePlayerController.CycleGolfClub` (`self.GolfController`) 0))))

(event `self.ReceiveTick`
  (params (DeltaSeconds :type "Float (single-precision)"))
  (bind (_returnvalue_roll _returnvalue_pitch _returnvalue_yaw) (`KismetMathLibrary.BreakRotator` (`self.GetControlRotation`)))
  ;[0.15 0.15 0.15 0.5 30] Tick
  (`|ExecutionSequence`
    (:`then_0`
      (`/Game/Blueprints/Player/BP_GolfGamePlayerController.CanShoot` (`self.GolfController`)
        (:`then`
          (bind _golfclub (`self.GolfClub`)
            (:`then`
              (`self.K2_SetActorRotation` _golfclub (`KismetMathLibrary.MakeRotator` 0.0 0.0 _returnvalue_yaw) false) ; Orientate Golf Club
            )
            (:`else`)))
        (:`else`)))
    (:`then_1`
      (`self.UpdatePredictSpline`))))

(event `self.ReceiveActorBeginOverlap`
  (params (OtherActor :type "Actor Object Reference"))
  (if (`self.ActorHasTag` OtherActor "Info")
    (`KismetArrayLibrary.Array_Add` (`self.CollectedInfoPanelActors`) OtherActor)
    (set `self.NewInfoPanel` true)
    (bind _returnvalue (`KismetArrayLibrary.Array_RemoveItem` (`/Game/Blueprints/Player/BP_GolfGamePlayerController.InfoPanels` (`self.GolfController`))))
    (if _returnvalue
      (`/Game/Blueprints/Player/BP_GolfGamePlayerController.UpdateInfoPanelTracker` (`self.GolfController`)))))

(event `TryCinematicCamera`
  ; Try to do cinematic camera
  (if (> (`KismetMathLibrary.VSize` (`SceneComponent.GetComponentVelocity` (`self.StaticMesh`))) 500.0)
    (`/Game/Blueprints/BP_GolfGameMode.SwitchPlayerCamera` (`self.GolfGame`) true)
    (set `self.IsCinematicOn` true)))

(event `FreezeBall`
  ; Freeze Ball
  (if (`KismetSystemLibrary.K2_IsTimerActiveHandle` (`self.GolfActiveHandle`))
    (`self.ShotComplete`))
  (`PrimitiveComponent.SetSimulatePhysics` (`self.StaticMesh`) false))

(event `StartOffsetTransition`
  (params (NewOffset :type "Vector Structure"))
  ; Animate Change Camera Offset
  (set `self.EndOffset` NewOffset)
  (set `self.StartOffset` (`SpringArmComponent.SocketOffset` (`self.SpringArm`)))
  (bind (_direction _offsetalpha) (`Timeline|CameraOffset` :!via `PlayFromStart`)
    (:`Update`
      (set `SpringArmComponent.SocketOffset` (`KismetMathLibrary.VLerp` (`self.StartOffset`) (`self.EndOffset`) _offsetalpha) (`self.SpringArm`)))))

(event `ShotComplete`
  ;[0.00209 0.7344 0.07098 0.5] Shot Complete
  (set `self.LastTransform` (`self.GetTransform`))
  (`KismetSystemLibrary.K2_ClearAndInvalidateTimerHandle` (`self.GolfActiveHandle`))
  (`PrimitiveComponent.SetSimulatePhysics` (`self.StaticMesh`) false)
  (`PrimitiveComponent.SetLinearDamping` (`self.StaticMesh`) 0.0)
  (`|ExecutionSequence`
    (:`then_0`
      (`/Game/Blueprints/BP_GolfGameMode.DoWind` (`self.GolfGame`))
      (`self.IsCinematicOn`
        (:`then`
          (`/Game/Blueprints/BP_GolfGameMode.SwitchPlayerCamera` (`self.GolfGame`) false))
        (:`else`)))
    (:`then_1`
      (`self.NewInfoPanel`
        (:`then`
          (bind _asplayer_hud (cast `/Game/Blueprints/UI/PlayerHUD` (`PlayerController.GetHUD` (`self.GolfController`))))
          (add `/Game/Blueprints/UI/InformationPanels/W_InfoPanelWidget.InfoClosed` (`/Game/Blueprints/UI/PlayerHUD.InfoPanelHUD` _asplayer_hud) (delegate `InfoPanelSequence`))
          (set `self.InfoCount` 0)
          (`self.InfoPanelSequence`))
        (:`else`
          (`/Game/Blueprints/Player/BP_GolfGamePlayerController.ResetGolfShot` (`self.GolfController`)))))))

(event `InfoPanelSequence`
  ;[0.00209 0.7344 0.07098 0.5] Shot Complete
  (if (>= (`self.InfoCount`) (`KismetArrayLibrary.Array_Length` (`self.CollectedInfoPanelActors`)))
    (`/Game/Blueprints/Player/BP_GolfGamePlayerController.ResetGolfShot` (`self.GolfController`))
    (`KismetArrayLibrary.Array_Clear` (`self.CollectedInfoPanelActors`))
    (else
      (bind _asbp_golf_game_mode (cast `/Game/Blueprints/BP_GolfGameMode` (`GameplayStatics.GetGameMode`)))
      (`/Game/Blueprints/BP_GolfGameMode.LockInputs` _asbp_golf_game_mode
        (:`then`
          _)
        (:`else`
          (`/Game/Blueprints/Components/BP_InfoPanelComponent.DisplayInfoPanel` (`self.BP_InfoPanelComponent`) (`|GetArrayItem` (`self.CollectedInfoPanelActors`) (`self.InfoCount`)) (`self.GetController`))))
      (set `self.NewInfoPanel` false)
      (`/Engine/EditorBlueprintResources/StandardMacros.IncrementInt` (`self.InfoCount`)))))

(fn `CanApplyDamping`
  (params (Grace :type "Float (double-precision)"))
  (returns (Check :type Boolean))
  (bind _outhit (`KismetSystemLibrary.LineTraceSingle` (`self.K2_GetActorLocation`) (+ (`self.K2_GetActorLocation`) (* (`KismetMathLibrary.Vector_Down`) 32.0)) "TraceTypeQuery1" true))
  (return (and (`self.BallFloored`) (> (`self.GroundFrictionTimer`) Grace) (> (.z (`.Normal` (`GameplayStatics.BreakHitResult` _outhit))) 0.995))))

(fn `GetSoundFromPhysMat`
  (params (PhysMat :type "PhysicalMaterial Object Reference"))
  (returns (Sound :type "SoundWave Object Reference"))
  (locals (PhysMatLocal :type "PhysicalMaterial Object Reference"))
  (bind _output_get (set `local.PhysMatLocal` PhysMat))
  (if (== _output_get "/Game/Materials/PhysicsMaterials/PM_Fairway.PM_Fairway")
    (return "/Game/Assets/Sounds/Golfball/MS_Impact_Solid.MS_Impact_Solid") ; Fairway - Solid
    (elif (== (`local.PhysMatLocal`) "/Game/Materials/PhysicsMaterials/PM_Rough.PM_Rough")
      (return "/Game/Assets/Sounds/Golfball/MS_Impact_Grass.MS_Impact_Grass") ; Rough - Grass
      (elif (== (`local.PhysMatLocal`) "/Game/Materials/PhysicsMaterials/PM_PuttingGreen.PM_PuttingGreen")
        (return "/Game/Assets/Sounds/Golfball/MS_Impact_Solid.MS_Impact_Solid") ; Putting Green
        (elif (== (`local.PhysMatLocal`) "/Game/Materials/PhysicsMaterials/PM_SandPit.PM_SandPit")
          (return "/Game/Assets/Sounds/Golfball/MS_Impact_Sand.MS_Impact_Sand") ; Sand Pit
          (else
            (return "/Game/Assets/Sounds/Golfball/MS_Impact_Solid.MS_Impact_Solid") ; Default - Solid
          ))))))

(fn `SpawnGolfClub`
  (bind (_returnvalue_location _returnvalue_rotation _returnvalue_scale) (`KismetMathLibrary.BreakTransform` (`self.GetTransform`)))
  (bind (_returnvalue_roll _returnvalue_pitch _returnvalue_yaw) (`KismetMathLibrary.BreakRotator` (`self.GetControlRotation`)))
  (bind _golfclub (`self.GolfClub`)
    (:`then`
      (`self.K2_DestroyActor` _golfclub))
    (:`else`
      _))
  (bind _returnvalue (`|SpawnActorFromClass` "/Game/Blueprints/Actor/BP_GolfClub.BP_GolfClub_C" (`KismetMathLibrary.MakeTransform` _returnvalue_location _returnvalue_rotation (* _returnvalue_scale 2.0)) "AlwaysSpawn" "OverrideRootScale" null null))
  (bind _output_get (set `self.GolfClub` _returnvalue))
  (`self.K2_SetActorRotation` _output_get (`KismetMathLibrary.MakeRotator` 0.0 0.0 _returnvalue_yaw) false))

(fn `UpdateGolfBallDamping`
  (params (PhysicsMaterial :type "PhysicalMaterial Object Reference (by ref)"))
  (bind _value (`BlueprintMapLibrary.Map_Find` (`self.PhysicsMaterialParameters`) (`BlueprintMapLibrary.Map_Find` (`self.PhysicsMaterialMap`) PhysicsMaterial)))
  (bind _check (`self.CanApplyDamping` (`.GracePeriod_5_09A1BACD44394939D78A74B9EA63A90F` (break `/Game/Blueprints/Structures/S_GroundTypeParameters` _value))))
  (if _check
    ;[0 0.15 0.01746 0.5] Ball Damping Rules:
    ; - After ball has been grounded for 1 second increase damping
    ; - Damping increase determined by surface type (e.g. rough stops faster)
    ; - If the ball's velocity is below a set value in the curve (500 units/s), then rapidly increase damping
    (set `self.BallStoppingForceMultiplier` (`.DampingMultiplier_9_C2C636D048D5404556919895627D80E6` (break `/Game/Blueprints/Structures/S_GroundTypeParameters` _value)))
    (set `self.BallStoppingForce` (+ (`self.BallStoppingForce`) (* (`self.BallStoppingForceMultiplier`) (`GameplayStatics.GetWorldDeltaSeconds`) (`CurveFloat.GetFloatValue` (`self.BallVelocityForceCurve`) (`KismetMathLibrary.VSize` (`self.GetVelocity`))))))
    (else
      (`self.BallFloored`
        (:`then`
          (set `self.GroundFrictionTimer` (+ (`self.GroundFrictionTimer`) (`GameplayStatics.GetWorldDeltaSeconds`))))
        (:`else`
          (set `self.GroundFrictionTimer` 0.0))))))

(fn `UserConstructionScript`)