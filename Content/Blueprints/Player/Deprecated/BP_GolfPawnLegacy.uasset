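; Deprecated golf player pawn Blueprint that handles camera hand-off and an intro camera move.
; TakeCameraControl switches the view target to a given actor and locks inputs; RestoreCamera returns the view to the pawn.
; When an intro is requested, RestoreCamera also starts the transition and unlocks inputs.
; The Transition timeline eases the spring arm's socket offset from IntroCamVector to zero by repeatedly lerping the current offset.
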(event `TakeCameraControl`
  (params (Actor :type "Actor Object Reference"))
  (`PlayerController.SetViewTargetWithBlend` (`PlayerState.GetPlayerController` (`Pawn.PlayerState` (`GameplayStatics.GetPlayerPawn` 0))) Actor 0.0 "VTBlend_Linear" 0.0 false)
  (set `self.bInputsLocked` true))

(event `RestoreCamera`
  (params (PlayIntroSequence :type Boolean))
  (`|ExecutionSequence`
    (:`then_0`
      (`PlayerController.SetViewTargetWithBlend` (`PlayerState.GetPlayerController` (`Pawn.PlayerState` (`GameplayStatics.GetPlayerPawn` 0))) self 0.0 "VTBlend_Linear" 0.0 false))
    (:`then_1`
      (if PlayIntroSequence
        (`self.DoIntroTransition`)
        (set `self.bInputsLocked` false)))))

(event `DoIntroTransition`
  (set `SpringArmComponent.SocketOffset` (`self.IntroCamVector`) (`self.SpringArm`))
  (bind (_direction _progress) (`Timeline|Transition` :!via `PlayFromStart`)
    (:`Update`
      (set `SpringArmComponent.SocketOffset` (`KismetMathLibrary.VLerp` (`SpringArmComponent.SocketOffset` (`self.SpringArm`)) (0.0 0.0 0.0) _progress) (`self.SpringArm`)))
    (:`Finished`
      (set `SpringArmComponent.SocketOffset` (0.0 0.0 0.0) (`self.SpringArm`)))))

(fn `UserConstructionScript`)