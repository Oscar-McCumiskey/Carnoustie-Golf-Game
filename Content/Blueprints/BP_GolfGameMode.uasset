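; Game mode for a golf game that tracks strokes against par, sets wind and switches between player and cinematic cameras.
; Strokes count down from each hole's par and map to par or bogey names.
; Wind is randomised at BeginPlay and passed to the HUD and ball.
; The cine camera jumps near the end hole and tracks the ball on a timer; a separate event hides PCG instanced meshes from minimap captures.
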(event Custom|OnStroke
  (bind _result (Math|Integer|DecrementInt (Variables|Default|GetCurStroke))
    (:%20%20
      (CallFunction|GetStrokeScoreDisplay _result))))

(event Custom|NewHoleReset
  (params (NewPar :type Integer))
  (bind _output_get (Variables|Default|SetCurPar NewPar))
  (Variables|Default|SetCurStroke _output_get))

(event Custom|SwitchPlayerCamera
  (params (UseCinematicCamera :type Boolean))
  (if UseCinematicCamera
    (Game|Player|SetViewTargetwithBlend (Variables|Default|GetPlayerController) (Variables|Default|GetCineCamera) 0.0 "VTBlend_Linear" 0.0 false)
    (bind _returnvalue (Actor|GetActorOfClass "/Game/Blueprints/Actor/BP_EndHole.BP_EndHole_C"))
    (CallFunction|DoRandomCineCamPosition (Transformation|GetActorLocation _returnvalue) 512.0)
    (bind _returnvalue_2 (Utilities|Time|SetTimerbyEvent (delegate Custom|CineCameraTick) 0.01 true))
    (Variables|Default|SetCineTimerHandle _returnvalue_2)
    (else
      (Game|Player|SetViewTargetwithBlend (Variables|Default|GetPlayerController) (Variables|Default|GetPlayerCamera) 0.0 "VTBlend_Linear" 0.0 false)
      (if (Utilities|Time|IsValidTimerHandle (Variables|Default|GetCineTimerHandle))
        (Utilities|Time|ClearandInvalidateTimerbyHandle (Variables|Default|GetCineTimerHandle))))))

(event Custom|DoWind
  ;[0.15 0.15 0.15 0.5] Wind Setup
  (Variables|Default|GetIsWindEnabled
    (:then
      (bind (_power _direction) (Default|RandomiseWind (Variables|Default|GetBP_Wind)))
      (bind _asplayer_hud (Utilities|Casting|CastToPlayerHUD (HUD|GetHUD (Game|GetPlayerController 0))))
      (Default|UpdateWind _asplayer_hud _power _direction)
      (bind _asbp_golf_ball (Utilities|Casting|CastToBP_GolfBall (Game|Player|GetPlayerPawn 0)))
      (Variables|/Game/Blueprints/Player/BP_GolfBall.BP_GolfBall_C|SetWindPower _asbp_golf_ball _power)
      (Variables|/Game/Blueprints/Player/BP_GolfBall.BP_GolfBall_C|SetWindDirection _asbp_golf_ball _direction))
    (:else)))

(event Custom|CineCameraTick
  (if (== (Pawn|GetViewTarget (Variables|Default|GetPlayerController)) (Variables|Default|GetCineCamera))
    (Transformation|SetActorRotation (Variables|Default|GetCineCamera) (Math|Rotator|FindLookatRotation (Transformation|GetActorLocation (Variables|Default|GetCineCamera)) (Transformation|GetActorLocation (Variables|Default|GetPlayerGolf))))))

(event Custom|ReturnToTimelineEvent_Event
  (Variables|Default|SetLockInputs true))

(event Custom|HideGrassOnMinimap
  (bind _outactors (Actor|GetAllActorsOfClass "/Script/PCG.PCGVolume"))
  (for _array_element _outactors
    (for _array_element_2 (Components|GetChildrenComponents (Variables|/Script/Engine.Brush|GetBrushComponent _array_element) false)
      (bind _asinstanced_static_mesh_component (Utilities|Casting|CastToInstancedStaticMeshComponent _array_element_2))
      (Class|PrimitiveComponent|SetHiddeninSceneCapture _asinstanced_static_mesh_component true))))

(event EventBeginPlay
  (bind _asbp_golf_ball (Utilities|Casting|CastToBP_GolfBall (Game|Player|GetPlayerPawn 0)))
  (bind _output_get (Variables|Default|SetPlayerGolf _asbp_golf_ball))
  (Utilities|FlowControl|Sequence
    (:then_0
      (Variables|Default|SetPlayerCamera (Components|GetOwner (Variables|/Script/CarnoustieGolfGame.GolfBallPawn|GetCamera _output_get)))
      (bind _returnvalue (Game|SpawnActorfromClass "/Game/Blueprints/BP_CineCamera.BP_CineCamera_C" (Math|Transform|MakeTransform "0, 0, 0" "0, 0, 0" "1.000000,1.000000,1.000000") "Undefined" "MultiplyWithRoot" 0 0))
      (Variables|Default|SetCineCamera _returnvalue)
      (bind _asbp_golf_game_player_controller (Utilities|Casting|CastToBP_GolfGamePlayerController (Game|GetPlayerController 0)))
      (Variables|Default|SetPlayerController _asbp_golf_game_player_controller)
      (Utilities|FlowControl|DelayUntilNextTick)
      (bind _asplayer_hud (Utilities|Casting|CastToPlayerHUD (HUD|GetHUD (Game|GetPlayerController 0))))
      (EventDispatchers|AssignReturntoTimelineEvent (Variables|/Game/Blueprints/UI/PlayerHUD.PlayerHUD_C|GetReturnTimelineHUD _asplayer_hud) (delegate Custom|ReturnToTimelineEvent_Event)))
    (:then_1
      (EventDispatchers|BindEventtoOnStroke _asbp_golf_ball (delegate Custom|OnStroke))
      (Utilities|FlowControl|DelayUntilNextTick)
      (CallFunction|DoWind))))

(fn ConstructionScript)

(fn GetStrokeScoreDisplay
  (params (Score :type Integer))
  (bind _returnvalue (Math|Integer|Absolute(Integer) Score))
  (bind _bogeynames (Variables|Default|GetBogeyNames))
  (bind _returnvalue_2 (- _returnvalue 1))
  (if (< Score 0) ; Went over Par
    (if (<= (Utilities|Array|Length _bogeynames) _returnvalue_2) ; Went over Bogeys
      (return (Utilities|String|StringToName (Utilities|String|Append "Quadruple Bogey +" (Utilities|String|ToString(Integer) (- _returnvalue_2 3))))) ; Return overscoring bogey
      (else
        (return (Utilities|Array|Get(acopy) _bogeynames _returnvalue_2)) ; Return Bogey names
      ))
    (else
      (return (Utilities|Array|Get(acopy) (Variables|Default|GetParNames) Score)) ; Return Par names
    )))

(fn DoRandomCineCamPosition
  (params (Point :type Vector) (Distance :type Float%20%28double-precision%29))
  (Transformation|SetWorldLocation (Variables|/Script/Engine.Actor|GetRootComponent (Variables|Default|GetCineCamera)) (+ (+ Point (* (Math|Vector|MakeVector (Math|Random|RandomFloatinRange -3.0 3.0) (Math|Random|RandomFloatinRange -3.0 3.0) 0.0) Distance)) (* (Math|Vector|VectorUp) 9.6e+02)) false false))