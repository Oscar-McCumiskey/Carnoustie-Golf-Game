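; Earth globe actor for the world pin map that keeps its material's city-light cycle aligned with the level's directional light.
; BeginPlay creates the dynamic material, finds the sun and sets the gradient band widths.
; With RotSun on, Tick advances a wrapping cycle that drives both sun yaw and the lights parameter.
; Otherwise, it derives the cycle from the yaw difference between Earth and sun; a toggle event flips the mode.
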(event `self.ReceiveBeginPlay`
  (bind _returnvalue (`PrimitiveComponent.CreateDynamicMaterialInstance` (`self.Earth`) 0 null "None"))
  (set `self.DynamicMaterial` _returnvalue)
  (bind _returnvalue_2 (`GameplayStatics.GetActorOfClass` "/Script/Engine.DirectionalLight"))
  (set `self.SunLight` _returnvalue_2)
  ; Set Earth Lights in correct starting rotation
  (`self.SetEarthLightCycleBasedOnSun`)
  (`MaterialInstanceDynamic.SetScalarParameterValue` (`self.DynamicMaterial`) "EarthLightsCycle" (- (`self.EarthLightsCycle`) (`self.BackGradientWidth`)))
  ; Earth Lights Width
  (`|ExecutionSequence`
    (:`then_0`
      (`MaterialInstanceDynamic.SetScalarParameterValue` (`self.DynamicMaterial`) "BackGradientWidth" (`self.BackGradientWidth`)))
    (:`then_1`
      (`MaterialInstanceDynamic.SetScalarParameterValue` (`self.DynamicMaterial`) "MainWidth" (`self.MainWidth`)))
    (:`then_2`
      (`MaterialInstanceDynamic.SetScalarParameterValue` (`self.DynamicMaterial`) "FrontGradientWidth" (`self.FrontGradientWidth`)))))

(event `ToggleRotSunEvent`
  (bind _output_get (set `self.RotSun` (not (`self.RotSun`))))
  (`KismetSystemLibrary.PrintString` (`KismetStringLibrary.Concat_StrStr` "Rot Sun = " (`KismetStringLibrary.Conv_BoolToString` _output_get))))

(event `self.ReceiveTick`
  (params (DeltaSeconds :type "Float (single-precision)"))
  (bind _sunlight (`self.SunLight`))
  (bind (_returnvalue_roll _returnvalue_pitch _returnvalue_yaw) (`KismetMathLibrary.BreakRotator` (`SceneComponent.K2_GetComponentRotation` (`self.Earth`))))
  (bind (_returnvalue_roll_2 _returnvalue_pitch_2) (`KismetMathLibrary.BreakRotator` (`self.K2_GetActorRotation` _sunlight)))
  (bind _returnvalue (+ (* (`self.SunSpeed`) DeltaSeconds) (`self.EarthLightsCycle`)))
  ;[0 0.6216 0.9479 0.5] Rotate Sun and Earth Lights
  (`self.RotSun`
    (:`then`
      (`/Engine/EditorBlueprintResources/StandardMacros.CompareFloat` _returnvalue 1.0
        (:`>`
          (set `self.EarthLightsCycle` 0.0 :!label _label))
        (:`==`
          (goto _label))
        (:`<`
          (set `self.EarthLightsCycle` _returnvalue)))
      (`self.K2_SetActorRotation` _sunlight (`KismetMathLibrary.MakeRotator` _returnvalue_roll_2 _returnvalue_pitch_2 (- (+ (`KismetMathLibrary.MapRangeClamped` (- 1.0 (`self.EarthLightsCycle`)) 0.0 1.0 0.0 360.0) _returnvalue_yaw) 180.0)) false)
      (`MaterialInstanceDynamic.SetScalarParameterValue` (`self.DynamicMaterial`) "EarthLightsCycle" (- (`self.EarthLightsCycle`) (`self.BackGradientWidth`))))
    (:`else`
      (`self.SetEarthLightCycleBasedOnSun`)
      (`MaterialInstanceDynamic.SetScalarParameterValue` (`self.DynamicMaterial`) "EarthLightsCycle" (- (`self.EarthLightsCycle`) (`self.BackGradientWidth`))))))

(fn `UserConstructionScript`)