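; Touch-driven camera pawn for the world pin map, viewing an Earth globe through a spring arm.
; Pinch zooms by changing clamped arm length, locking inputs until both fingers lift.
; After an idle delay following touch, Tick slowly yaws the pawn, with Alt+F as a debug toggle.
; Mouse-wheel input rescales turn sensitivity in proportion to arm length; Tick prints pinch sensitivity for debugging.
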(event Custom|SetPawnNotIdle
  ;[0.004038 0.15 0 0.5] Pawn Idle Logic
  (Variables|Idle|SetIsPawnIdle false)
  (Utilities|Time|ClearandInvalidateTimerbyHandle (stale Custom|PawnIdleTimerEvent _returnvalue)))

(event Custom|PawnIdleTimerEvent
  ;[0.004038 0.15 0 0.5] Pawn Idle Logic
  (Utilities|FlowControl|Sequence
    (:then_0
      (Variables|Idle|SetIsPawnIdle false)
      (Utilities|Time|ClearandInvalidateTimerbyHandle (stale _returnvalue)))
    (:then_1
      (bind _returnvalue (Utilities|Time|SetTimerbyEvent (delegate Custom|SetPawnToIdle) (Variables|Idle|GetIdleDelay))))))

(event Custom|SetPawnToIdle
  ;[0.004038 0.15 0 0.5] Pawn Idle Logic
  (Variables|Idle|SetIsPawnIdle true))

(event Input|EnhancedActionEvents|EnhancedInputActionIA_MouseWheel
  (params (ActionValue :type Boolean) (ElapsedSeconds :type Float%20%28double-precision%29) (TriggeredSeconds :type Float%20%28double-precision%29) (InputAction :type Input%20Action%20Object%20Reference :default "/Game/Blueprints/Player/Inputs/MouseInput/IA_MouseWheel.IA_MouseWheel"))
  ;[0.15 0.15 0.15 0.5] Change Turn Sensitivity based on Zoom
  (Variables|Default|SetTurnSensitivity (* (Variables|/Script/Engine.SpringArmComponent|GetTargetArmLength (Variables|Default|GetSpringArm)) (Math|Float|SafeDivide (Variables|Defaults|GetDefault%20Turn%20Sensitivity) (Variables|Defaults|GetDefault%20Arm%20Length)))))

(event Input|EnhancedActionEvents|EnhancedInputActionIA_Pinch
  (params (ActionValue :type Float%20%28double-precision%29) (ElapsedSeconds :type Float%20%28double-precision%29) (TriggeredSeconds :type Float%20%28double-precision%29) (InputAction :type Input%20Action%20Object%20Reference :default "/Game/Blueprints/Player/Inputs/TouchInput/IA_Pinch.IA_Pinch"))
  (bind _returnvalue (Viewport|GetViewportSize))
  (bind (_min _max) (Utilities|GetMinMaxArmLength))
  (bind _springarm (Variables|Default|GetSpringArm))
  (bind _returnvalue_2 (Math|Vector|Distance2D(Vector) :V2 _returnvalue))
  (bind _returnvalue_3 (/ ActionValue _returnvalue_2))
  ;[1 0.4728 0.000518 0.5] Pinch Zoom
  (:Triggered
    (Math|Float|CompareFloat _returnvalue_3 (Variables|Touch|Pinch|GetPinchValue)
      (:>
        (bind _value (Utilities|ValueonBranch (/ _returnvalue_3 (Variables|Touch|Pinch|GetPinchValue)) (/ (Variables|Touch|Pinch|GetPinchValue) _returnvalue_3) :!label _label)
          (:1
            (bind _value_2 (Utilities|ValueonBranch (- (Variables|/Script/Engine.SpringArmComponent|GetTargetArmLength _springarm) (* _value (Variables|Touch|Pinch|GetPinchZoomSensitivity))) (+ (* _value (Variables|Touch|Pinch|GetPinchZoomSensitivity)) (Variables|/Script/Engine.SpringArmComponent|GetTargetArmLength _springarm)) :!label _label_2)
              (:1
                _)
              (:2
                _))
            (Variables|/Script/Engine.SpringArmComponent|SetTargetArmLength _springarm (Math|Float|Clamp(Float) _value_2 _min _max))
            (Variables|Touch|Pinch|SetPinchValue _returnvalue_3))
          (:2
            (goto _label_2 Option2))))
      (:<
        (goto _label Option2))))
  (:Started
    (Variables|Touch|Pinch|SetHasPinchStarted true)
    (Variables|Default|SetbInputsLocked true)
    (Variables|Touch|Pinch|SetPinchValue 0.0)))

(event EventBeginPlay
  ;[0.15 0.15 0.15 0.5] Begin Play
  (Variables|Defaults|SetDefault%20Turn%20Sensitivity (Variables|Default|GetTurnSensitivity))
  (Variables|Defaults|SetDefault%20Arm%20Length (Variables|/Script/Engine.SpringArmComponent|GetTargetArmLength (Variables|Default|GetSpringArm)))
  (bind _asbp_earth (Utilities|Casting|CastToBP_Earth (Variables|/Script/Engine.ChildActorComponent|GetChildActor (Variables|Default|GetEarthGlobe))))
  (Variables|Default|SetEarth _asbp_earth)
  (Variables|Default|SetGlobePawnSizeDelta (.X (Math|Vector|BreakVector (- (Transformation|GetWorldScale (Variables|Default|GetEarthGlobe)) (Transformation|GetActorScale3D))))))

(event EventTick
  (params (DeltaSeconds :type Float%20%28single-precision%29))
  (Utilities|FlowControl|Sequence
    (:then_0
      ;[0 0.5004 1 0.5] Idle Rotate
      (if (and (Variables|Idle|GetIsPawnIdle) (Variables|Default|GetRotPawn))
        (Transformation|AddActorLocalRotation (Math|Rotator|MakeRotator 0.0 0.0 (* DeltaSeconds (Variables|Idle|GetPawnRotSpeed))) false false)))
    (:then_1
      ;[0.151 0 0 0.5] If two fingers were down, enable input after both are up
      (Variables|Touch|Pinch|GetHasPinchStarted
        (:then
          (if (not (or (Variables|Touch|GetIsTouch1Down) (Variables|Touch|GetIsTouch2Down)))
            (Variables|Touch|Pinch|SetHasPinchStarted false)
            (Class|GolfBallPawn|SetPrevTouchVector (Input|EnhancedActionValues|GetIA_Touch1))
            (Variables|Default|SetbInputsLocked false)))
        (:else)))
    (:then_2
      (Development|PrintString (Utilities|String|Append "Sensitivity = " (Utilities|String|ToString(Float) (Variables|Touch|Pinch|GetPinchZoomSensitivity))) true true "(R=0.000000,G=0.660000,B=1.000000,A=1.000000)" 0.0))))

(event Input|KeyboardEvents|DebugKeyAltF
  (params (Key :type Key%20Structure :default "None") (ActionValue :type Input%20Action%20Value%20Structure))
  ;[0 0.9059 1 0.5] Freeze Rotation
  (:Pressed
    (bind _output_get (Variables|Default|SetRotPawn (not (Variables|Default|GetRotPawn))))
    (Development|PrintString (Utilities|String|Append "Rot Pawn = " (Utilities|String|ToString(Boolean) _output_get)))))

(event Input|TouchEvents|Touch1
  (params (Key :type Key%20Structure :default "None"))
  ;[0.004038 0.15 0 0.5] Pawn Idle Logic
  (:Pressed
    (Variables|Idle|SetIsPawnIdle false)
    (Utilities|Time|ClearandInvalidateTimerbyHandle (stale _returnvalue)))
  (:Released
    (bind _returnvalue (Utilities|Time|SetTimerbyEvent (delegate Custom|SetPawnToIdle) (Variables|Idle|GetIdleDelay)))))

(event Input|TouchEvents|Touch1
  (params (Key :type Key%20Structure :default "None"))
  ;[0.15 0.15 0.15 0.5] Is Touches 1 & 2 Pressed
  (:Pressed
    (Variables|Touch|SetIsTouch1Down true))
  (:Released
    (Variables|Touch|SetIsTouch1Down false)))

(event Input|TouchEvents|Touch2
  (params (Key :type Key%20Structure :default "None"))
  ;[0.15 0.15 0.15 0.5] Is Touches 1 & 2 Pressed
  (:Pressed
    (Variables|Touch|SetIsTouch2Down true))
  (:Released
    (Variables|Touch|SetIsTouch2Down false)))

(fn ConstructionScript)