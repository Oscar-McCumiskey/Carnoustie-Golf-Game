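; WorldPinMapHUD sets up the on-screen UI for the world pin map level and handles the return to the timeline level.
; On BeginPlay it adds the pin map, return-to-timeline and fade widgets to the viewport, then plays a fade-out.
; The return widget's event triggers a fade-in, whose finish callback opens L_Timeline, so the level change waits for the transition.
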(event `self.ReceiveBeginPlay`
  (`|ExecutionSequence`
    (:`then_0`
      (bind _returnvalue (`|CreateWidget` "/Game/Blueprints/WorldPinMap/W_WorldPinMap.W_WorldPinMap_C"))
      (bind _output_get (set `self.WorldPinMapUI` _returnvalue))
      (`UserWidget.AddToViewport` _output_get 0))
    (:`then_1`
      ; Return to timeline
      (bind _returnvalue_2 (`|CreateWidget` "/Game/Blueprints/UI/BP_ReturnToTimeline.BP_ReturnToTimeline_C"))
      (bind _output_get_2 (set `self.ReturnTimelineHUD` _returnvalue_2))
      (`UserWidget.AddToViewport` _output_get_2 0)
      (add `/Game/Blueprints/UI/BP_ReturnToTimeline.ReturnToTimelineEvent` _output_get_2 (delegate `EventReturnToTimeline`)))
    (:`then_2`
      ; Fade effect
      (bind _returnvalue_3 (`|CreateWidget` "/Game/Blueprints/UI/W_Fade.W_Fade_C"))
      (bind _output_get_3 (set `self.Fade Widget` _returnvalue_3))
      (`Widget.SetRenderScale` _output_get_3 (`WidgetLayoutLibrary.GetViewportSize`))
      (`UserWidget.AddToViewport` _output_get_3 0)
      (`/Game/Blueprints/UI/W_Fade.PlayFadeOut` _output_get_3 0.5))))

(event `EventReturnToTimeline`
  ; Return to timeline
  (`/Game/Blueprints/UI/W_Fade.PlayFadeIn` (`self.Fade Widget`) 1.0)
  (add `/Game/Blueprints/UI/W_Fade.OnFadeInFinish` (`self.Fade Widget`) (delegate `OnFadeFinish_Event`)))

(event `OnFadeFinish_Event`
  ; Return to timeline
  (`GameplayStatics.OpenLevel` "L_Timeline"))

(fn `UserConstructionScript`)